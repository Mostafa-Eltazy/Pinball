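; BP_Plunger is a plunger actor, apparently for launching a ball, that can be charged and released.
; ChargePlunger plays a timeline that lerps the plunger mesh along its local Y axis to pull it out of rest.
; StopCharge halts the timeline and quickly moves the mesh with MoveComponentTo.
; GetballspawnLocation converts a local ball position to world space through the actor's transform.
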(event `ChargePlunger`
  (bind (_direction _alphacharge) (`Timeline|ChargeTimeline` :!via `PlayFromStart` :!label _label)
    (:`Update`
      (`SceneComponent.K2_SetRelativeLocation` (`self.PlungerMesh`) (`KismetMathLibrary.VLerp` (0.0 0.0 0.0) (0.0 150.0 0.0) _alphacharge) false false))))

(event `StopCharge`
  (`|ExecutionSequence`
    (:`then_0`
      (goto _label :!via `Stop`))
    (:`then_1`
      (`KismetSystemLibrary.MoveComponentTo` (`self.PlungerMesh`) (0.0 0.0 0.0) (struct) false false 0.1))))

(fn `GetballspawnLocation`
  (returns (ballspawnlocation :type "Vector Structure"))
  (return (`KismetMathLibrary.TransformLocation` (`self.GetTransform`) (`self.balllocation`))))

(fn `UserConstructionScript`)