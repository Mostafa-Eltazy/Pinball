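; Pinball flipper actor that swings between a rest and a raised rotation as a left or right paddle.
; The construction script derives both rotations from Fliptype, poses the Flipper component at rest and mirrors its X scale for the right side.
; Flip and Flop events move the component between those rotations over FlipTime, with Flip also playing an attached sound.
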(event `self.ReceiveBeginPlay`)

(event `Flip`
  (`KismetSystemLibrary.MoveComponentTo` (`self.Flipper`) (0.0 0.0 0.0) (`self.endRotation`) false false (`self.FlipTime`))
  (`GameplayStatics.SpawnSoundAttached` "/Game/Assets/Sounds/PinballFlibber_Cue.PinballFlibber_Cue" (`self.Flipper`) "None" (0.0 0.0 0.0) (struct) "KeepRelativeOffset" false 0.25 0.25 0.0 null null))

(event `Flop`
  (`KismetSystemLibrary.MoveComponentTo` (`self.Flipper`) (0.0 0.0 0.0) (`self.startRotation`) false false (`self.FlipTime`)))

(fn `UserConstructionScript`
  (set `self.startRotation` (select `/Game/BlueBrint/FlipType` (`self.fliptype`) :`NewEnumerator0` (struct :`Yaw` 20.0) :`NewEnumerator1` (struct :`Yaw` -20.0) :!type "Rotator Structure"))
  (set `self.endRotation` (select `/Game/BlueBrint/FlipType` (`self.fliptype`) :`NewEnumerator0` (struct :`Yaw` -20.0) :`NewEnumerator1` (struct :`Yaw` 20.0) :!type "Rotator Structure"))
  (`SceneComponent.K2_SetRelativeRotation` (`self.Flipper`) (`self.startRotation`) false false)
  (switch `/Game/BlueBrint/FlipType` (`self.fliptype`)
    (:`NewEnumerator1`
      (`SceneComponent.SetRelativeScale3D` (`self.Flipper`) (-1.0 1.0 1.0)))))